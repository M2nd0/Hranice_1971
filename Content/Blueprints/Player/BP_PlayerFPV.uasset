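; First-person player character that drives a linear quest line of talking to NPCs and collecting items.
; It creates the mission, interact and collect widgets, and handles movement, look and jump, with the first Drive input setting the first mission.
; Interact passes the Quest stage to overlapping NPCs through BPI_Talk.
; Pick line-traces from the camera for tagged key, toolboxes or fuel, each gated by quest stage, updating counters and completion flags.
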(event Custom|InteractTextOn
  (UserInterface|Viewport|AddtoViewport (Variables|Default|GetInteract) 0))

(event Custom|InteractTextOff
  (Widget|RemovefromParent (Variables|Default|GetInteract)))

(event EventBeginPlay
  (bind _returnvalue (UserInterface|CreateWidget "/Game/Blueprints/Widgets/WP_UI.WP_UI_C" (Game|GetPlayerController 0)))
  (bind _output_get (Variables|Default|SetMissionText _returnvalue))
  (UserInterface|Viewport|AddtoViewport _output_get 0)
  (bind _returnvalue_2 (UserInterface|CreateWidget "/Game/Blueprints/Widgets/WP_Interact.WP_Interact_C"))
  (Variables|Default|SetInteract _returnvalue_2)
  (bind _returnvalue_3 (UserInterface|CreateWidget "/Game/Blueprints/Widgets/WP_Collect.WP_Collect_C"))
  (Variables|Default|SetCollect _returnvalue_3)
  (Audio|PlaySound2D "/Game/Sounds/lescvrčekk.lescvrčekk" 0.5 1.0 0.0 0 0))

(event Input|ActionEvents|InputActionJump
  (params (Key :type Key%20Structure :default "None"))
  (:Pressed
    (Character|Jump)))

(event Input|ActionEvents|InputActionPick
  (params (Key :type Key%20Structure :default "None"))
  (bind _toolboxes (Variables|Default|GetToolboxes))
  (bind _fuel (Variables|Default|GetFuel))
  (bind _camera (Variables|Default|GetCamera))
  (bind _returnvalue (Transformation|GetWorldLocation _camera))
  (:Pressed
    (bind _outhit (Collision|LineTraceByChannel _returnvalue (+ _returnvalue (* (Math|Vector|GetForwardVector (Transformation|GetWorldRotation _camera)) (Math|Conversions|ToVector(Float) 1.5e+03))) "TraceTypeQuery1" true 0 "ForDuration"))
    (if (Actor|ActorHasTag (.hitactor _outhit) "Item_key")
      (if (== (Variables|Default|GetQuest) 2)
        (Variables|Default|SetKeyCollected true)
        (Actor|DestroyActor (.hitactor _outhit))
        (Audio|PlaySound2D "/Game/Sounds/klice-_AudioTrimmer_com_.klice-_AudioTrimmer_com_" 1.0 1.0 0.0 0 0)
        (Variables|Default|SetQuestCompleted_0 true))
      (elif (Actor|ActorHasTag (.hitactor _outhit) "Item_toolbox")
        (if (== (Variables|Default|GetQuest) 3)
          (Math|Integer|IncrementInt _toolboxes
            (:%20%20
              (Variables|/Script/UMG.TextBlock|SetText (Variables|/Game/Blueprints/Widgets/WP_UI.WP_UI_C|GetToolbox_count (Variables|Default|GetMissionText)) (Utilities|Text|ToText(Integer) _toolboxes))
              (Actor|DestroyActor (.hitactor _outhit))
              (if (>= (Variables|Default|GetToolboxes) 4)
                (Variables|Default|SetQuestCompleted_1 true)))))
        (elif (Actor|ActorHasTag (.hitactor _outhit) "Item_fuel")
          (if (== (Variables|Default|GetQuest) 4)
            (Math|Integer|IncrementInt _fuel
              (:%20%20
                (Variables|/Script/UMG.TextBlock|SetText (Variables|/Game/Blueprints/Widgets/WP_UI.WP_UI_C|GetFuel_count (Variables|Default|GetMissionText)) (Utilities|Text|ToText(Integer) _fuel))
                (Actor|DestroyActor (.hitactor _outhit))
                (if (>= (Variables|Default|GetFuel) 2)
                  (Variables|Default|SetQuestCompleted_2 true))))))))))

(event Input|ActionEvents|InputActionInteract
  (params (Key :type Key%20Structure :default "None"))
  (:Pressed
    (for _array_element (Collision|GetOverlappingActors "/Game/Blueprints/NPC/BP_NPC.BP_NPC_C" :!class /Script/Engine.Actor)
      (if (Utilities|DoesObjectImplementInterface _array_element "/Game/Blueprints/NPC/BPI_Talk.BPI_Talk_C")
        (Class|BPITalk|Talk(Message) _array_element (Variables|Default|GetQuest))))))

(event Input|AxisEvents|InputAxisDrive
  (params (AxisValue :type Float%20%28single-precision%29))
  (Pawn|Input|AddMovementInput (Math|Vector|GetForwardVector (Variables|Default|GetCamera)) AxisValue false)
  (Utilities|FlowControl|DoOnce false
    (:Completed
      (CallFunction|UpdateMission "Find the mechanic and talk to him."))))

(event Input|AxisEvents|InputAxisRotate
  (params (AxisValue :type Float%20%28single-precision%29))
  (Pawn|Input|AddControllerYawInput AxisValue))

(event Input|AxisEvents|InputAxisLookup
  (params (AxisValue :type Float%20%28single-precision%29))
  (Pawn|Input|AddControllerPitchInput AxisValue))

(event Input|AxisEvents|InputAxisTurn
  (params (AxisValue :type Float%20%28single-precision%29))
  (Pawn|Input|AddMovementInput (Math|Vector|GetRightVector (Variables|Default|GetCamera)) AxisValue false))

(fn ConstructionScript)

(fn UpdateMission
  (params (MissionTexxt :type String))
  (Rendering|Components|TextRender|SetText (Variables|/Game/Blueprints/Widgets/WP_UI.WP_UI_C|GetQuestText (Variables|Default|GetMissionText)) (Utilities|Text|ToText(String) MissionTexxt))
  (Math|Integer|IncrementInt (Variables|Default|GetQuest)))
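; BP_PlayerCar is a player-controlled car that drives and steers through CharacterMovement.
; The Drive axis adds movement along the inverted right vector of the `We` component, and Turn yaws that component only while the car has velocity.
; Tick stores the current speed and reapplies max speed, acceleration (Zrychleni) and braking deceleration (Zpomaleni) every frame.
; Equivalent FloatingPawnMovement setters remain unconnected.
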(event EventTick
  (params (DeltaSeconds :type Float%20%28single-precision%29))
  (bind _charactermovement (Variables|Character|GetCharacterMovement))
  (Variables|Default|SetSpeed (Math|Vector|VectorLength (Transformation|GetVelocity)))
  (Variables|/Script/Engine.CharacterMovementComponent|SetMaxWalkSpeed _charactermovement (Variables|Default|GetMaxSpeed))
  (Variables|/Script/Engine.CharacterMovementComponent|SetMaxAcceleration _charactermovement (Variables|Default|GetZrychleni))
  (Variables|/Script/Engine.CharacterMovementComponent|SetBrakingDecelerationWalking _charactermovement (Variables|Default|GetZpomaleni)))

(event Input|AxisEvents|InputAxisDrive
  (params (AxisValue :type Float%20%28single-precision%29))
  (Pawn|Input|AddMovementInput (Math|Vector|GetRightVector (Variables|Default|Getwe)) (* AxisValue -1.0) false))

(event Input|AxisEvents|InputAxisTurn
  (params (AxisValue :type Float%20%28single-precision%29))
  (if (not (<= (Math|Vector|VectorLength (Transformation|GetVelocity)) 0.001))
    (Transformation|AddLocalRotation (Variables|Default|Getwe) (Math|Rotator|MakeRotator 0.0 0.0 (* AxisValue -1.0)) false false)))

(fn ConstructionScript)
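; BP_NPC is a quest-giver NPC that steps the player through fetch missions ending in "Cross the border!".
; Sphere overlap toggles the player's interact prompt, and Talk advances WP_Dialog lines per quest stage, gated by BP_PlayerFPV completion flags, then updates the mission.
; The final stage reuses the fourth stage's dialog and completion flag.
; Separately, StaticMesh overlap spawns BP_Car and calls Possess with no pawn specified.
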(event OnComponentBeginOverlap(StaticMesh)
  (params (OverlappedComponent :type Primitive%20Component%20Object%20Reference) (OtherActor :type Actor%20Object%20Reference) (OtherComp :type Primitive%20Component%20Object%20Reference) (OtherBodyIndex :type Integer) (bFromSweep :type Boolean) (SweepResult :type Hit%20Result%20Structure%20%28by%20ref%29))
  (Utilities|Casting|CastToBP_PlayerFPV OtherActor)
  (Development|PrintString "Hello")
  (Game|SpawnActorfromClass "/Game/Blueprints/Items/BP_Car.BP_Car_C" (Transformation|GetActorTransform (Variables|Default|GetSpawn)) "Undefined" "MultiplyWithRoot" 0 0)
  (Pawn|Possess (Game|GetPlayerController 0)))

(event OnComponentEndOverlap(Sphere)
  (params (OverlappedComponent :type Primitive%20Component%20Object%20Reference) (OtherActor :type Actor%20Object%20Reference) (OtherComp :type Primitive%20Component%20Object%20Reference) (OtherBodyIndex :type Integer))
  (bind _asbp_player_fpv (Utilities|Casting|CastToBP_PlayerFPV OtherActor))
  (Default|InteractTextOff _asbp_player_fpv))

(event OnComponentBeginOverlap(Sphere)
  (params (OverlappedComponent :type Primitive%20Component%20Object%20Reference) (OtherActor :type Actor%20Object%20Reference) (OtherComp :type Primitive%20Component%20Object%20Reference) (OtherBodyIndex :type Integer) (bFromSweep :type Boolean) (SweepResult :type Hit%20Result%20Structure%20%28by%20ref%29))
  (bind _asbp_player_fpv (Utilities|Casting|CastToBP_PlayerFPV OtherActor))
  (Variables|Default|SetAs%20BP%20Player%20FPV _asbp_player_fpv)
  (Default|InteractTexton _asbp_player_fpv))

(event Custom|NesplnenyQuest
  (CallFunction|DialogText "Nejdrive spln quest")
  (Utilities|FlowControl|Delay 3.0)
  (CallFunction|DialogText))

(event EventTalk
  (params (Quest :type Integer))
  (bind _dialog2 (Variables|Default|GetDialog2))
  (bind _dialog1 (Variables|Default|GetDialog1))
  (bind _as_bp_player_fpv (Variables|Default|GetAs%20BP%20Player%20FPV))
  (bind _as_bp_player_fpv_2 (Variables|Default|GetAs%20BP%20Player%20FPV))
  (bind _dialog3 (Variables|Default|GetDialog3))
  (bind _as_bp_player_fpv_3 (Variables|Default|GetAs%20BP%20Player%20FPV))
  (bind _dialog4 (Variables|Default|GetDialog4))
  (bind _dialog4_2 (Variables|Default|GetDialog4))
  (bind _as_bp_player_fpv_4 (Variables|Default|GetAs%20BP%20Player%20FPV))
  (UserInterface|Viewport|AddtoViewport (stale EventBeginPlay _output_get) 0)
  (switch int Quest
    (:1
      (Math|Integer|IncrementInt (Variables|Default|GetDialogNumber)
        (:%20%20
          (if (< (Variables|Default|GetDialogNumber) (Utilities|Array|Length _dialog1))
            (CallFunction|DialogText (Utilities|Array|Get(acopy) _dialog1 (Variables|Default|GetDialogNumber)))
            (else
              (Math|Integer|IncrementInt (Variables|Default|GetQuest)
                (:%20%20
                  (CallFunction|DialogText)
                  (Default|UpdateMission _as_bp_player_fpv_2 "Find car key")
                  (Variables|Default|SetDialogNumber -1))))))))
    (:2
      (if (Variables|/Game/Blueprints/Player/BP_PlayerFPV.BP_PlayerFPV_C|GetQuestCompleted_0 (Variables|Default|GetAs%20BP%20Player%20FPV))
        (Math|Integer|IncrementInt (Variables|Default|GetDialogNumber)
          (:%20%20
            (if (< (Variables|Default|GetDialogNumber) (Utilities|Array|Length _dialog2))
              (CallFunction|DialogText (Utilities|Array|Get(acopy) _dialog2 (Variables|Default|GetDialogNumber)))
              (else
                (Math|Integer|IncrementInt (Variables|Default|GetQuest)
                  (:%20%20
                    (CallFunction|DialogText)
                    (Default|UpdateMission _as_bp_player_fpv_2 "Find 4 toolboxes")
                    (Variables|Default|SetDialogNumber -1)))))))
        (else
          (CallFunction|NesplnenyQuest))))
    (:3
      (if (Variables|/Game/Blueprints/Player/BP_PlayerFPV.BP_PlayerFPV_C|GetQuestCompleted_1 (Variables|Default|GetAs%20BP%20Player%20FPV))
        (Math|Integer|IncrementInt (Variables|Default|GetDialogNumber)
          (:%20%20
            (if (< (Variables|Default|GetDialogNumber) (Utilities|Array|Length _dialog3))
              (CallFunction|DialogText (Utilities|Array|Get(acopy) _dialog3 (Variables|Default|GetDialogNumber)))
              (else
                (Math|Integer|IncrementInt (Variables|Default|GetQuest)
                  (:%20%20
                    (CallFunction|DialogText)
                    (Default|UpdateMission _as_bp_player_fpv_3 "Find 4 metal plates")
                    (Variables|/Game/Blueprints/Player/BP_PlayerFPV.BP_PlayerFPV_C|SetToolboxes _as_bp_player_fpv_3 0)
                    (Variables|Default|SetDialogNumber -1)))))))
        (else
          (CallFunction|NesplnenyQuest))))
    (:4
      (if (Variables|/Game/Blueprints/Player/BP_PlayerFPV.BP_PlayerFPV_C|GetQuestCompleted_2 (Variables|Default|GetAs%20BP%20Player%20FPV))
        (Math|Integer|IncrementInt (Variables|Default|GetDialogNumber)
          (:%20%20
            (if (< (Variables|Default|GetDialogNumber) (Utilities|Array|Length _dialog4_2))
              (CallFunction|DialogText (Utilities|Array|Get(acopy) _dialog4_2 (Variables|Default|GetDialogNumber)))
              (else
                (Math|Integer|IncrementInt (Variables|Default|GetQuest)
                  (:%20%20
                    (CallFunction|DialogText)
                    (Default|UpdateMission _as_bp_player_fpv_4 "Find 2 fuel cans")
                    (Variables|/Game/Blueprints/Player/BP_PlayerFPV.BP_PlayerFPV_C|SetPlates _as_bp_player_fpv_4 0)
                    (Variables|Default|SetDialogNumber -1)))))))
        (else
          (CallFunction|NesplnenyQuest))))
    (:5
      (if (Variables|/Game/Blueprints/Player/BP_PlayerFPV.BP_PlayerFPV_C|GetQuestCompleted_2 (Variables|Default|GetAs%20BP%20Player%20FPV))
        (Math|Integer|IncrementInt (Variables|Default|GetDialogNumber)
          (:%20%20
            (if (< (Variables|Default|GetDialogNumber) (Utilities|Array|Length _dialog4))
              (CallFunction|DialogText (Utilities|Array|Get(acopy) _dialog4 (Variables|Default|GetDialogNumber)))
              (else
                (Math|Integer|IncrementInt (Variables|Default|GetQuest)
                  (:%20%20
                    (CallFunction|DialogText)
                    (Default|UpdateMission _as_bp_player_fpv "Cross the border!")
                    (Variables|/Game/Blueprints/Player/BP_PlayerFPV.BP_PlayerFPV_C|SetPlates _as_bp_player_fpv 0)
                    (Variables|Default|SetDialogNumber -1)))))))
        (else
          (CallFunction|NesplnenyQuest))))))

(event EventBeginPlay
  (bind _returnvalue (UserInterface|CreateWidget "/Game/Blueprints/Widgets/WP_Dialog.WP_Dialog_C" (Game|GetPlayerController 0)))
  (bind _output_get (Variables|Default|SetDialogProm _returnvalue)))

(fn ConstructionScript)

(fn DialogText
  (params (Text :type String))
  (Variables|/Script/UMG.TextBlock|SetText (Variables|/Game/Blueprints/Widgets/WP_Dialog.WP_Dialog_C|GetTextBlock_0 (Variables|Default|GetDialogProm)) (Utilities|Text|ToText(String) Text)))